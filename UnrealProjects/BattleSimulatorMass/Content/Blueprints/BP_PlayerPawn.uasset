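; Player pawn for a battle simulation, acting as a keyboard control layer for running battles and switching between test levels.
; Enter and Backspace cast the game mode to BP_BattleSimGameMode and call its start and restart functions.
; Number keys open separate Battle levels whose name suffixes climb mostly by doubling, apparently battle sizes.
; Tick prints an on-screen hint for the start and reset keys every frame.
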(event `self.ReceiveTick`
  (params (DeltaSeconds :type "Float (single-precision)"))
  (`KismetSystemLibrary.PrintString` "Enter: Start \nBackspace: Reset" true false (struct :`G` 0.66 :`B` 1.0 :`A` 1.0) 0.0))

(event `Key|Enter` :consume false :paused true
  (params (Key :type "Key Structure"))
  (:`Pressed`
    (bind _asbp_battle_sim_game_mode (cast `/Game/Blueprints/BP_BattleSimGameMode` (`GameplayStatics.GetGameMode`)))
    (`BattleSimGameMode.StartSimulation` _asbp_battle_sim_game_mode)))

(event `Key|BackSpace` :consume false :paused true
  (params (Key :type "Key Structure"))
  (:`Pressed`
    (bind _asbp_battle_sim_game_mode (cast `/Game/Blueprints/BP_BattleSimGameMode` (`GameplayStatics.GetGameMode`)))
    (`BattleSimGameMode.Restart` _asbp_battle_sim_game_mode)))

(event `Key|Zero` :consume false :paused true
  (params (Key :type "Key Structure"))
  (:`Pressed`
    (`GameplayStatics.OpenLevelBySoftObjectPtr` "/Game/Levels/Battle_1.Battle_1")))

(event `Key|One` :consume false :paused true
  (params (Key :type "Key Structure"))
  (:`Pressed`
    (`GameplayStatics.OpenLevelBySoftObjectPtr` "/Game/Levels/Battle_100.Battle_100")))

(event `Key|Two` :consume false :paused true
  (params (Key :type "Key Structure"))
  (:`Pressed`
    (`GameplayStatics.OpenLevelBySoftObjectPtr` "/Game/Levels/Battle_200.Battle_200")))

(event `Key|Three` :consume false :paused true
  (params (Key :type "Key Structure"))
  (:`Pressed`
    (`GameplayStatics.OpenLevelBySoftObjectPtr` "/Game/Levels/Battle_400.Battle_400")))

(event `Key|Four` :consume false :paused true
  (params (Key :type "Key Structure"))
  (:`Pressed`
    (`GameplayStatics.OpenLevelBySoftObjectPtr` "/Game/Levels/Battle_800.Battle_800")))

(event `Key|Five` :consume false :paused true
  (params (Key :type "Key Structure"))
  (:`Pressed`
    (`GameplayStatics.OpenLevelBySoftObjectPtr` "/Game/Levels/Battle_1600.Battle_1600")))

(event `Key|Six` :consume false :paused true
  (params (Key :type "Key Structure"))
  (:`Pressed`
    (`GameplayStatics.OpenLevelBySoftObjectPtr` "/Game/Levels/Battle_3200.Battle_3200")))

(event `Key|Seven` :consume false :paused true
  (params (Key :type "Key Structure"))
  (:`Pressed`
    (`GameplayStatics.OpenLevelBySoftObjectPtr` "/Game/Levels/Battle_6400.Battle_6400")))

(event `Key|Eight` :consume false :paused true
  (params (Key :type "Key Structure"))
  (:`Pressed`
    (`GameplayStatics.OpenLevelBySoftObjectPtr` "/Game/Levels/Battle_12800.Battle_12800")))

(fn `UserConstructionScript`)