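; Player pawn that serves as the keyboard control for a battle simulation, printing its key hints every tick.
; Number keys reload the Battle level with URL options that set preset unit counts and spawn ranges.
; Enter asks BP_BattleSimGameMode to spawn units, or start the simulation once spawned, and Backspace restarts it.
; A SpawnUnits function can also set the unit manager's count and spawn, restarting instead if already spawned.
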(event `self.ReceiveTick`
  (params (DeltaSeconds :type "Float (single-precision)"))
  (`KismetSystemLibrary.PrintString` "0-8: Choose preset \nEnter: Start \nBackspace: Reset" true false (struct :`G` 0.66 :`B` 1.0 :`A` 1.0) 0.0))

(event `Key|Enter` :consume false :paused true
  (params (Key :type "Key Structure"))
  (:`Pressed`
    (bind _asbp_battle_sim_game_mode (cast `/Game/Blueprints/BP_BattleSimGameMode` (`GameplayStatics.GetGameMode`)))
    (if (`BattleSimGameMode.HasSpawned` _asbp_battle_sim_game_mode)
      (`BattleSimGameMode.StartSimulation` _asbp_battle_sim_game_mode)
      (else
        (`BattleSimGameMode.StartSpawning` _asbp_battle_sim_game_mode)))))

(event `Key|BackSpace` :consume false :paused true
  (params (Key :type "Key Structure"))
  (:`Pressed`
    (bind _asbp_battle_sim_game_mode (cast `/Game/Blueprints/BP_BattleSimGameMode` (`GameplayStatics.GetGameMode`)))
    (`BattleSimGameMode.Restart` _asbp_battle_sim_game_mode)))

(event `Key|Zero` :consume false :paused true
  (params (Key :type "Key Structure"))
  (:`Pressed`
    (`GameplayStatics.OpenLevelBySoftObjectPtr` "/Game/Levels/Battle.Battle" true "SpawnCount=1?SpawnPosRange=3500")))

(event `Key|One` :consume false :paused true
  (params (Key :type "Key Structure"))
  (:`Pressed`
    (`GameplayStatics.OpenLevelBySoftObjectPtr` "/Game/Levels/Battle.Battle" true "SpawnCount=100?SpawnPosRange=3500")))

(event `Key|Two` :consume false :paused true
  (params (Key :type "Key Structure"))
  (:`Pressed`
    (`GameplayStatics.OpenLevelBySoftObjectPtr` "/Game/Levels/Battle.Battle" true "SpawnCount=200?SpawnPosRange=3500")))

(event `Key|Three` :consume false :paused true
  (params (Key :type "Key Structure"))
  (:`Pressed`
    (`GameplayStatics.OpenLevelBySoftObjectPtr` "/Game/Levels/Battle.Battle" true "SpawnCount=400?SpawnPosRange=4000")))

(event `Key|Four` :consume false :paused true
  (params (Key :type "Key Structure"))
  (:`Pressed`
    (`GameplayStatics.OpenLevelBySoftObjectPtr` "/Game/Levels/Battle.Battle" true "SpawnCount=800?SpawnPosRange=5000")))

(event `Key|Five` :consume false :paused true
  (params (Key :type "Key Structure"))
  (:`Pressed`
    (`GameplayStatics.OpenLevelBySoftObjectPtr` "/Game/Levels/Battle.Battle" true "SpawnCount=1600?SpawnPosRange=6000")))

(event `Key|Six` :consume false :paused true
  (params (Key :type "Key Structure"))
  (:`Pressed`
    (`GameplayStatics.OpenLevelBySoftObjectPtr` "/Game/Levels/Battle.Battle" true "SpawnCount=3200?SpawnPosRange=8000")))

(event `Key|Seven` :consume false :paused true
  (params (Key :type "Key Structure"))
  (:`Pressed`
    (`GameplayStatics.OpenLevelBySoftObjectPtr` "/Game/Levels/Battle.Battle" true "SpawnCount=6400?SpawnPosRange=10000")))

(event `Key|Eight` :consume false :paused true
  (params (Key :type "Key Structure"))
  (:`Pressed`
    (`GameplayStatics.OpenLevelBySoftObjectPtr` "/Game/Levels/Battle.Battle" true "SpawnCount=12800?SpawnPosRange=14000")))

(fn `SpawnUnits`
  (params (Count :type Integer))
  (bind _asbp_battle_sim_game_mode (cast `/Game/Blueprints/BP_BattleSimGameMode` (`GameplayStatics.GetGameMode`)))
  (if (`BattleSimGameMode.HasSpawned` _asbp_battle_sim_game_mode)
    (`BattleSimGameMode.Restart` _asbp_battle_sim_game_mode)
    (else
      (set `UnitManager.SpawnCount` Count (`BattleSimGameMode.GetUnitManager` _asbp_battle_sim_game_mode))
      (`BattleSimGameMode.StartSpawning` _asbp_battle_sim_game_mode))))

(fn `UserConstructionScript`)